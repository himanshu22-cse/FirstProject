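; Player controller Blueprint that shows and dismisses the pause menu with animations.
; It overrides the display and remove events, casting the inherited or stored PauseMenu reference to play its forward or reverse animation, then calling the parent implementations.
; Display sets the menu visible before the parent call, while removal waits briefly after it and also sets visibility to Visible rather than hiding it.
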(event `self.DisplayPauseMenu`
  (bind _aspause_menu (cast `/Game/HUD/PauseMenu` (`self.PauseMenu`)))
  (`/Game/HUD/PauseMenu.PlayMenuAnimation` _aspause_menu)
  (`Widget.SetVisibility` (`self.PauseMenu`) "Visible")
  (`parent.DisplayPauseMenu`))

(event `self.RemovePauseMenu`
  (bind _aspause_menu (cast `/Game/HUD/PauseMenu` (`self.PauseMenu`)))
  (`/Game/HUD/PauseMenu.PlayReverseAnimation` _aspause_menu)
  (`parent.RemovePauseMenu`)
  (`KismetSystemLibrary.Delay` 0.25)
  (`Widget.SetVisibility` (`self.PauseMenu`) "Visible"))

(fn `UserConstructionScript`)